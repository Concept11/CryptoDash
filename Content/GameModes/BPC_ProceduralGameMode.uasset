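; Game mode for an endless runner that procedurally chains BPC_ThreePlane tiles, runs a timed score and drives a moon powerup.
; Tiles spawn at the previous tile's attach transform, and passing index thresholds raises difficulty, which periodically increases obstacle limits and player speed.
; Obstacles roll against difficulty and are rejected when nearby tiles are too crowded or form impossible combinations.
; The powerup lifts the gravity-free player through a delayed loop, then sets NavWalking.
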(event Custom|E_ExecuteMoonPowerup
  (params (PlayerCharacter :type BPC%20Player%20Character%20Object%20Reference))
  (Utilities|MExecuteMoonPowerup PlayerCharacter
    (:%20
      (Pawn|Components|CharacterMovement|SetMovementMode (Variables|/Script/Engine.Character|GetCharacterMovement PlayerCharacter) "MOVE_NavWalking" 0))))

(event EventBeginPlay
  (bind _asbpc_player_character (Utilities|Casting|CastToBPC_PlayerCharacter (Pawn|GetControlledPawn (Game|GetPlayerController 0))))
  (if (Utilities|IsValid _asbpc_player_character)
    (Utilities|FlowControl|Sequence
      (:then_0
        (CallFunction|PopulateDifficultyThresholds))
      (:then_1
        (bind _returnvalue (UserInterface|CreateWidget "/Game/Widgets/BPC_ProceduralWidget.BPC_ProceduralWidget_C" (Game|GetPlayerController 0)))
        (UserInterface|Viewport|AddtoViewport _returnvalue 0)
        (Variables|Default|SetProceduralWidget _returnvalue))
      (:then_2
        (Utilities|Time|SetTimerbyFunctionName self "UpdateScore" 0.2 true))
      (:then_3
        (Variables|/Script/Engine.CharacterMovementComponent|SetMaxWalkSpeed (Variables|/Script/Engine.Character|GetCharacterMovement _asbpc_player_character) (Variables|Default|GetCharacterSpeed)))
      (:then_4
        (for _index (range 0 9)
          (CallFunction|AddFloorTile _index true))))))

(fn ConstructionScript)

(fn AddFloorTile
  (params (Index :type Integer) (Initial%20Tiles? :type Boolean))
  (if Initial%20Tiles?
    (LocalVariables|SetLocalIndex Index)
    (else
      (LocalVariables|SetLocalIndex (+ Index 10))))
  (bind _threeplane (CallFunction|GetThreePlanefromIndex (+ Index 8)))
  (Variables|Default|SetBeforeThreePlane _threeplane)
  (bind _increasedifficulty_ (Updates|UpdateDifficultyIndex (Variables|Default|GetCurrentThreePlane)))
  (if _increasedifficulty_
    (bind _output_get (Variables|Default|SetDifficultyIndex (+ (Variables|Default|GetDifficultyIndex) 1)))
    (Updates|UpdateObstacleDifficultyIndex _output_get)
    (Updates|UpdateCharacterSpeed _output_get))
  (bind (_obstacletype _tiletype) (Calculations|CalculateObstacle (LocalVariables|GetLocalIndex) (Variables|Default|GetDifficultyIndex)))
  (bind _returnvalue (Game|SpawnActorfromClass "/Game/BPC_ThreePlane.BPC_ThreePlane_C" (Variables|Default|GetNextSpawnTransform) "Undefined" 0 (LocalVariables|GetLocalIndex) (Variables|Default|GetDifficultyIndex) _obstacletype _tiletype (Variables|Default|GetCharacterSpeed) 0))
  (Utilities|Array|Add (Variables|Default|GetThreePlaneArray) _returnvalue)
  (bind _attachtransform (Default|FGetAttachTransform _returnvalue))
  (Variables|Default|SetNextSpawnTransform _attachtransform)
  (Variables|Default|SetCurrentThreePlane _returnvalue))

(fn UpdateDifficultyIndex
  (params (CurrentThreePlane :type BPC%20Three%20Plane%20Object%20Reference))
  (if (Utilities|IsValid CurrentThreePlane)
    (return (Utilities|Array|ContainsItem (Variables|Default|GetDifficultyThresholds) (Variables|/Game/BPC_ThreePlane.BPC_ThreePlane_C|GetIndex CurrentThreePlane)))))

(fn PopulateDifficultyThresholds
  (for _index (range 1 10)
    (Utilities|Array|Add (Variables|Default|GetDifficultyThresholds) (* _index 100)))
  (for _index_2 (range 1 10)
    (Utilities|Array|Add (Variables|Default|GetDifficultyThresholds) (+ 1000 (* _index_2 250))))
  (for _index_3 (range 1 10)
    (Utilities|Array|Add (Variables|Default|GetDifficultyThresholds) (+ 3500 (* _index_3 500)))))

(fn CalculateObstacle
  (params (Index :type Integer) (DifficultyIndex :type Integer))
  (if (> Index 9)
    (if (<= (Math|Random|RandomIntegerinRange 0 100) DifficultyIndex)
      (bind _toodifficult_ (Calculations|CalculateNumberOfObstacles Index))
      (if _toodifficult_
        (Development|PrintString "Too difficult")
        (else
          (bind _possibleimpossibility_ (Calculations|CalculateImpossibility))
          (if _possibleimpossibility_
            (Development|PrintString "Impossibility")
            (else
              (return (Utilities|Select :Index (Math|Random|RandomInteger (- (|GetNumEnumEntries) 1)) :Option%200 (Utilities|Enum|LiteralenumE_ObstacleType "NewEnumerator0") :Option%201 (Utilities|Enum|LiteralenumE_ObstacleType "NewEnumerator3") :Option%202 (Utilities|Enum|LiteralenumE_ObstacleType "NewEnumerator4") :Option%203 (Utilities|Enum|LiteralenumE_ObstacleType "NewEnumerator5")) (Utilities|Select :Index (Math|Random|RandomInteger (- (|GetNumEnumEntries) 1)) :Option%200 (Utilities|Enum|LiteralenumE_TileType "NewEnumerator0") :Option%201 (Utilities|Enum|LiteralenumE_TileType "NewEnumerator1") :Option%202 (Utilities|Enum|LiteralenumE_TileType "NewEnumerator2")))))))))
  (return "NewEnumerator2" "NewEnumerator3"))

(fn GetThreePlanefromIndex
  (params (Index :type Integer))
  (for _array_element (Variables|Default|GetThreePlaneArray)
    (if (Utilities|IsValid _array_element)
      (if (== Index (Variables|/Game/BPC_ThreePlane.BPC_ThreePlane_C|GetIndex _array_element))
        (return _array_element))))
  (return _array_element))

(fn CalculateImpossibility
  (bind _beforethreeplane (Variables|Default|GetBeforeThreePlane))
  (bind _currentthreeplane (Variables|Default|GetCurrentThreePlane))
  (if (or (and (Utilities|Enum|Equal(Enum) (Variables|/Game/BPC_ThreePlane.BPC_ThreePlane_C|GetTileType _beforethreeplane) "NewEnumerator0") (Utilities|Enum|Equal(Enum) (Variables|/Game/BPC_ThreePlane.BPC_ThreePlane_C|GetTileType _currentthreeplane) "NewEnumerator1")) (and (Utilities|Enum|Equal(Enum) (Variables|/Game/BPC_ThreePlane.BPC_ThreePlane_C|GetTileType _beforethreeplane) "NewEnumerator2") (Utilities|Enum|Equal(Enum) (Variables|/Game/BPC_ThreePlane.BPC_ThreePlane_C|GetTileType _currentthreeplane) "NewEnumerator1")))
    (return true)
    (else
      (return false))))

(fn CalculateNumberOfObstacles
  (params (Index :type Integer))
  (for _array_element (Variables|Default|GetThreePlaneArray)
    (if (Utilities|IsValid _array_element)
      (if (>= (Variables|/Game/BPC_ThreePlane.BPC_ThreePlane_C|GetIndex _array_element) (- Index 9))
        (if (Utilities|Enum|NotEqual(Enum) (Variables|/Game/BPC_ThreePlane.BPC_ThreePlane_C|GetTileType _array_element) "NewEnumerator3")
          (LocalVariables|SetLocalNumberOfObstacles (+ (LocalVariables|GetLocalNumberOfObstacles) 1))))))
  (if (Math|Integer|InRange(Integer) (LocalVariables|GetLocalNumberOfObstacles) 0 (Variables|Default|GetObstacleDifficultyIndex))
    (return false)
    (else
      (return true))))

(fn UpdateObstacleDifficultyIndex
  (params (DifficultyIndex :type Integer))
  (if (Math|Boolean|ORBoolean (== DifficultyIndex 31) (== DifficultyIndex 33) (== DifficultyIndex 35) (== DifficultyIndex 40) (== DifficultyIndex 45) (== DifficultyIndex 50))
    (Variables|Default|SetObstacleDifficultyIndex (+ (Variables|Default|GetObstacleDifficultyIndex) 1))))

(fn UpdateCharacterSpeed
  (params (DifficultyIndex :type Integer))
  (if (Math|Boolean|ORBoolean (== DifficultyIndex 31) (== DifficultyIndex 33) (== DifficultyIndex 35) (== DifficultyIndex 40) (== DifficultyIndex 45) (== DifficultyIndex 50))
    (Variables|Default|SetCharacterSpeed (+ (Variables|Default|GetCharacterSpeed) 4e+02))
    (bind _asbpc_player_character (Utilities|Casting|CastToBPC_PlayerCharacter (Pawn|GetControlledPawn (Game|GetPlayerController 0))))
    (Variables|/Script/Engine.CharacterMovementComponent|SetMaxWalkSpeed (Variables|/Script/Engine.Character|GetCharacterMovement _asbpc_player_character) (Variables|Default|GetCharacterSpeed))))

(fn UpdateScore
  (bind _result (Math|Float|IncrementFloat (Variables|Default|GetScore))
    (:%20%20
      (Default|SetScoreText (Variables|Default|GetProceduralWidget) _result))))