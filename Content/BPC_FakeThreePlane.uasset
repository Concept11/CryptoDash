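; Three-plane row piece that colors its left, center and right tiles in alternating white and orange.
; On BeginPlay it reads PreviousPlane's center tile and inverts the pattern, forming a checkerboard across consecutive rows.
; It stores each tile's data and applies the materials to the three planes, doing nothing without a PreviousPlane.
; SetTileTexture repeats the tile selection without applying materials.
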(event EventBeginPlay
  (if (!= (Variables|Default|GetPreviousPlane) 0)
    (if (== (.Texture (Utilities|Struct|BreakS_TileData (Variables|/Game/BPC_ThreePlane.BPC_ThreePlane_C|GetCenterTile (Variables|Default|GetPreviousPlane)))) "/Game/Materials/M_White.M_White")
      (Variables|Default|SetLeftTile (Utilities|Struct|MakeS_TileData "NewEnumerator0" "NewEnumerator2" "/Game/Materials/M_White.M_White"))
      (Variables|Default|SetCenterTile (Utilities|Struct|MakeS_TileData "NewEnumerator0" "NewEnumerator2" "/Game/Materials/M_Orange.M_Orange"))
      (Variables|Default|SetRightTile (Utilities|Struct|MakeS_TileData "NewEnumerator0" "NewEnumerator2" "/Game/Materials/M_White.M_White"))
      (else
        (Variables|Default|SetLeftTile (Utilities|Struct|MakeS_TileData "NewEnumerator0" "NewEnumerator2" "/Game/Materials/M_Orange.M_Orange"))
        (Variables|Default|SetCenterTile (Utilities|Struct|MakeS_TileData "NewEnumerator0" "NewEnumerator2" "/Game/Materials/M_White.M_White"))
        (Variables|Default|SetRightTile (Utilities|Struct|MakeS_TileData "NewEnumerator0" "NewEnumerator2" "/Game/Materials/M_Orange.M_Orange"))))
    (Rendering|Material|SetMaterial (Variables|Default|GetLeftPlane) 0 (.texture (Variables|Default|GetLeftTile)))
    (Rendering|Material|SetMaterial (Variables|Default|GetCenterPlane) 0 (.texture (Variables|Default|GetCenterTile)))
    (Rendering|Material|SetMaterial (Variables|Default|GetRightPlane) 0 (.texture (Variables|Default|GetRightTile)))))

(fn ConstructionScript)

(fn SetTileTexture
  (if (!= (Variables|Default|GetPreviousPlane) 0)
    (if (== (.Texture (Utilities|Struct|BreakS_TileData (Variables|/Game/BPC_ThreePlane.BPC_ThreePlane_C|GetCenterTile (Variables|Default|GetPreviousPlane)))) "/Game/Materials/M_White.M_White")
      (Variables|Default|SetLeftTile (Utilities|Struct|MakeS_TileData "NewEnumerator0" "NewEnumerator2" "/Game/Materials/M_White.M_White"))
      (Variables|Default|SetCenterTile (Utilities|Struct|MakeS_TileData "NewEnumerator0" "NewEnumerator2" "/Game/Materials/M_Orange.M_Orange"))
      (Variables|Default|SetRightTile (Utilities|Struct|MakeS_TileData "NewEnumerator0" "NewEnumerator2" "/Game/Materials/M_White.M_White"))
      (else
        (Variables|Default|SetLeftTile (Utilities|Struct|MakeS_TileData "NewEnumerator0" "NewEnumerator2" "/Game/Materials/M_Orange.M_Orange"))
        (Variables|Default|SetCenterTile (Utilities|Struct|MakeS_TileData "NewEnumerator0" "NewEnumerator2" "/Game/Materials/M_White.M_White"))
        (Variables|Default|SetRightTile (Utilities|Struct|MakeS_TileData "NewEnumerator0" "NewEnumerator2" "/Game/Materials/M_Orange.M_Orange"))))))