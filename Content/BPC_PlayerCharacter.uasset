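; BPC_PlayerCharacter is an auto-running player character that dies on hitting track obstacles.
; Tick constantly pushes it along world forward, since only control roll feeds the direction, and Space jumps.
; Tick also raises gravity scale while airborne for faster falls, restoring it on the ground.
; CubeCollision overlaps destroy the character when the hit component matches a hack, bear, candle or fork component on a BPC_ThreePlane.
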(event OnComponentBeginOverlap(CubeCollision)
  (params (OverlappedComponent :type Primitive%20Component%20Object%20Reference) (OtherActor :type Actor%20Object%20Reference) (OtherComp :type Primitive%20Component%20Object%20Reference) (OtherBodyIndex :type Integer) (bFromSweep :type Boolean) (SweepResult :type Hit%20Result%20Structure%20%28by%20ref%29))
  (bind _asbpc_three_plane (Utilities|Casting|CastToBPC_ThreePlane OtherActor))
  (if (Math|Boolean|ORBoolean (== (Variables|/Game/BPC_ThreePlane.BPC_ThreePlane_C|GetLeftHackCollision _asbpc_three_plane) (.hitcomponent SweepResult)) (== (Variables|/Game/BPC_ThreePlane.BPC_ThreePlane_C|GetCenterHackCollision _asbpc_three_plane) (.hitcomponent SweepResult)) (== (Variables|/Game/BPC_ThreePlane.BPC_ThreePlane_C|GetRightHackCollision _asbpc_three_plane) (.hitcomponent SweepResult)) (== (Variables|/Game/BPC_ThreePlane.BPC_ThreePlane_C|GetLeftBear _asbpc_three_plane) (.hitcomponent SweepResult)) (== (Variables|/Game/BPC_ThreePlane.BPC_ThreePlane_C|GetRightBear _asbpc_three_plane) (.hitcomponent SweepResult)) (== (Variables|/Game/BPC_ThreePlane.BPC_ThreePlane_C|GetLeftCandle _asbpc_three_plane) (.hitcomponent SweepResult)) (== (Variables|/Game/BPC_ThreePlane.BPC_ThreePlane_C|GetCenterCandle _asbpc_three_plane) (.hitcomponent SweepResult)) (== (Variables|/Game/BPC_ThreePlane.BPC_ThreePlane_C|GetRightCandle _asbpc_three_plane) (.hitcomponent SweepResult)) (== (Variables|/Game/BPC_ThreePlane.BPC_ThreePlane_C|GetLeftFork _asbpc_three_plane) (.hitcomponent SweepResult)) (== (Variables|/Game/BPC_ThreePlane.BPC_ThreePlane_C|GetCenterFork _asbpc_three_plane) (.hitcomponent SweepResult)) (== (Variables|/Game/BPC_ThreePlane.BPC_ThreePlane_C|GetRightFork _asbpc_three_plane) (.hitcomponent SweepResult)))
    (Actor|DestroyActor)))

(event EventTick
  (params (DeltaSeconds :type Float%20%28single-precision%29))
  (bind _charactermovement (Variables|Character|GetCharacterMovement))
  (Utilities|FlowControl|Sequence
    (:then_0
      (Pawn|Input|AddMovementInput (Math|Vector|GetForwardVector (Math|Rotator|MakeRotator (.Roll (Math|Rotator|BreakRotator (Pawn|GetControlRotation :!class /Script/Engine.Pawn))) 0.0 0.0)) 1.0 false))
    (:then_1
      (if (AI|Components|NavMovement|IsFalling _charactermovement)
        (Variables|/Script/Engine.CharacterMovementComponent|SetGravityScale _charactermovement 1e+01)
        (else
          (Variables|/Script/Engine.CharacterMovementComponent|SetGravityScale _charactermovement 1.0))))))

(event Input|KeyboardEvents|SpaceBar
  (params (Key :type Key%20Structure))
  (:Pressed
    (Character|Jump)))

(fn ConstructionScript)