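; Three-lane floor tile for a procedural runner that sets up and runs one obstacle on BeginPlay: Hack, Candle, Fork or Bear.
; TileType picks the lane; timelines fade the hacked plane or move the props, with speed-scaled random delays for forks and bears.
; Decorative side candles get random heights and grey materials, and bear tiles flash the planes red.
; When the player leaves EndTrigger, it has the game mode add a tile, then destroys itself.
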(event OnComponentEndOverlap(EndTrigger)
  (params (OverlappedComponent :type Primitive%20Component%20Object%20Reference) (OtherActor :type Actor%20Object%20Reference) (OtherComp :type Primitive%20Component%20Object%20Reference) (OtherBodyIndex :type Integer))
  (Utilities|Casting|CastToBPC_PlayerCharacter OtherActor)
  (if (Variables|Default|GetNewSpawn?)
    (Variables|Default|SetNewSpawn? false)
    (bind _asbpc_procedural_game_mode (Utilities|Casting|CastToBPC_ProceduralGameMode (Game|GetGameMode)))
    (Default|AddFloorTile _asbpc_procedural_game_mode (Variables|Default|GetIndex) false)
    (Utilities|FlowControl|Delay 1.0)
    (Actor|DestroyActor)))

(event EventBeginPlay
  (Initialization|FInitializeLocations)
  (Initialization|FInitializeFakeCandles)
  (switch Utilities|FlowControl|Switch|SwitchonE_ObstacleType (Variables|Default|GetObstacleType)
    (:NewEnumerator0
      (|G_ExecuteHackObstacle (Variables|Default|GetTileType)))
    (:NewEnumerator3
      (|G_ExecuteCandleObstacle (Variables|Default|GetTileType)))
    (:NewEnumerator4
      (bind _delay (CallFunction|FCalculateForkDelay (Variables|Default|GetCharacterSpeed)))
      (|G_ExecuteForkObstacle (Variables|Default|GetTileType) _delay))
    (:NewEnumerator5
      (bind _delay_2 (CallFunction|FCalculateBearDelay (Variables|Default|GetCharacterSpeed)))
      (|G_ExecuteBearObstacle (Variables|Default|GetTileType) _delay_2))))

(fn ConstructionScript)

(fn FGetAttachTransform
  (return (Transformation|GetWorldTransform (Variables|Default|GetAttachPoint))))

(fn FCalculateForkDelay
  (params (CharacterSpeed :type Float%20%28single-precision%29))
  (switch string (Utilities|String|ToString(Float) CharacterSpeed)
    (:1600.0
      (LocalVariables|SetLocalDelay (Math|Random|RandomFloatinRange 1.6 2.2)))
    (:2000.0
      (LocalVariables|SetLocalDelay (Math|Random|RandomFloatinRange 1.3 1.8)))
    (:2400.0
      (LocalVariables|SetLocalDelay (Math|Random|RandomFloatinRange 0.9 1.4)))
    (:2800.0
      (LocalVariables|SetLocalDelay (Math|Random|RandomFloatinRange 0.7 1.2)))
    (:3200.0
      (LocalVariables|SetLocalDelay (Math|Random|RandomFloatinRange 0.6 1.0)))
    (:3600.0
      (LocalVariables|SetLocalDelay (Math|Random|RandomFloatinRange 0.5 0.8)))
    (:4000.0
      (LocalVariables|SetLocalDelay (Math|Random|RandomFloatinRange 0.4 0.75))))
  (return (LocalVariables|GetLocalDelay)))

(fn FCalculateBearDelay
  (params (CharacterSpeed :type Float%20%28single-precision%29))
  (switch string (Utilities|String|ToString(Float) CharacterSpeed)
    (:1600.0
      (LocalVariables|SetLocalDelay (Math|Random|RandomFloatinRange 1.4 2.2)))
    (:2000.0
      (LocalVariables|SetLocalDelay (Math|Random|RandomFloatinRange 1.0 1.7)))
    (:2400.0
      (LocalVariables|SetLocalDelay (Math|Random|RandomFloatinRange 0.7 1.3)))
    (:2800.0
      (LocalVariables|SetLocalDelay (Math|Random|RandomFloatinRange 0.5 1.0)))
    (:3200.0
      (LocalVariables|SetLocalDelay (Math|Random|RandomFloatinRange 0.35 0.9)))
    (:3600.0
      (LocalVariables|SetLocalDelay (Math|Random|RandomFloatinRange 0.25 0.75)))
    (:4000.0
      (LocalVariables|SetLocalDelay (Math|Random|RandomFloatinRange 0.15 0.65))))
  (return (LocalVariables|GetLocalDelay)))

(fn FInitializeFakeCandles
  (bind _fakerightcandle1 (Variables|Default|GetFakeRightCandle1))
  (bind _fakerightcandle2 (Variables|Default|GetFakeRightCandle2))
  (bind _fakeleftcandle2 (Variables|Default|GetFakeLeftCandle2))
  (bind _fakeleftcandle1 (Variables|Default|GetFakeLeftCandle1))
  (Transformation|SetRelativeLocation (Variables|Default|GetFakeRightCandle1) (Math|Vector|MakeVector 0.0 8e+02 (Math|Random|RandomFloatinRange -1.4e+03 -8e+02)) false false)
  (Transformation|SetRelativeLocation (Variables|Default|GetFakeRightCandle2) (Math|Vector|MakeVector 0.0 1.2e+03 (Math|Random|RandomFloatinRange -1e+03 -5e+02)) false false)
  (Transformation|SetRelativeLocation (Variables|Default|GetFakeLeftCandle1) (Math|Vector|MakeVector 0.0 -8e+02 (Math|Random|RandomFloatinRange -1.4e+03 -8e+02)) false false)
  (Transformation|SetRelativeLocation (Variables|Default|GetFakeLeftCandle2) (Math|Vector|MakeVector 0.0 -1.2e+03 (Math|Random|RandomFloatinRange -1e+03 -5e+02)) false false)
  (switch int (Math|Random|RandomIntegerinRange 0 2)
    (:0
      (Rendering|Material|SetMaterial _fakerightcandle1 0 "/Game/Materials/M_Grey1.M_Grey1"))
    (:1
      (Rendering|Material|SetMaterial _fakerightcandle1 0 "/Game/Materials/M_Grey2.M_Grey2"))
    (:2
      (Rendering|Material|SetMaterial _fakerightcandle1 0 "/Game/Materials/M_Grey3.M_Grey3")))
  (switch int (Math|Random|RandomIntegerinRange 0 2)
    (:0
      (Rendering|Material|SetMaterial _fakerightcandle2 0 "/Game/Materials/M_Grey1.M_Grey1"))
    (:1
      (Rendering|Material|SetMaterial _fakerightcandle2 0 "/Game/Materials/M_Grey2.M_Grey2"))
    (:2
      (Rendering|Material|SetMaterial _fakerightcandle2 0 "/Game/Materials/M_Grey3.M_Grey3")))
  (switch int (Math|Random|RandomIntegerinRange 0 2)
    (:0
      (Rendering|Material|SetMaterial _fakeleftcandle1 0 "/Game/Materials/M_Grey1.M_Grey1"))
    (:1
      (Rendering|Material|SetMaterial _fakeleftcandle1 0 "/Game/Materials/M_Grey2.M_Grey2"))
    (:2
      (Rendering|Material|SetMaterial _fakeleftcandle1 0 "/Game/Materials/M_Grey3.M_Grey3")))
  (switch int (Math|Random|RandomIntegerinRange 0 2)
    (:0
      (Rendering|Material|SetMaterial _fakeleftcandle2 0 "/Game/Materials/M_Grey1.M_Grey1"))
    (:1
      (Rendering|Material|SetMaterial _fakeleftcandle2 0 "/Game/Materials/M_Grey2.M_Grey2"))
    (:2
      (Rendering|Material|SetMaterial _fakeleftcandle2 0 "/Game/Materials/M_Grey3.M_Grey3"))))

(fn FSetPlanesRed
  (Rendering|Material|SetMaterial (Variables|Default|GetRightPlane) 0 "/Game/Materials/M_Red1.M_Red1")
  (Rendering|Material|SetMaterial (Variables|Default|GetCenterPlane) 0 "/Game/Materials/M_Red1.M_Red1")
  (Rendering|Material|SetMaterial (Variables|Default|GetLeftPlane) 0 "/Game/Materials/M_Red1.M_Red1")
  (Rendering|Material|SetMaterial (Variables|Default|GetFakeLeftPlane1) 0 "/Game/Materials/M_Red1.M_Red1")
  (Rendering|Material|SetMaterial (Variables|Default|GetFakeLeftPlane2) 0 "/Game/Materials/M_Red1.M_Red1")
  (Rendering|Material|SetMaterial (Variables|Default|GetFakeRightPlane1) 0 "/Game/Materials/M_Red1.M_Red1")
  (Rendering|Material|SetMaterial (Variables|Default|GetFakeRightPlane2) 0 "/Game/Materials/M_Red1.M_Red1"))

(fn FSetPlanesWhite
  (Rendering|Material|SetMaterial (Variables|Default|GetRightPlane) 0 "/Game/Materials/M_White.M_White")
  (Rendering|Material|SetMaterial (Variables|Default|GetCenterPlane) 0 "/Game/Materials/M_White.M_White")
  (Rendering|Material|SetMaterial (Variables|Default|GetLeftPlane) 0 "/Game/Materials/M_White.M_White")
  (Rendering|Material|SetMaterial (Variables|Default|GetFakeLeftPlane1) 0 "/Game/Materials/M_White.M_White")
  (Rendering|Material|SetMaterial (Variables|Default|GetFakeLeftPlane2) 0 "/Game/Materials/M_White.M_White")
  (Rendering|Material|SetMaterial (Variables|Default|GetFakeRightPlane1) 0 "/Game/Materials/M_White.M_White")
  (Rendering|Material|SetMaterial (Variables|Default|GetFakeRightPlane2) 0 "/Game/Materials/M_White.M_White"))

(fn FInitializeLocations
  (Variables|Locations|SetLeftCandleLocation (Variables|/Script/Engine.SceneComponent|GetRelativeLocation (Variables|Default|GetLeftCandle)))
  (Variables|Locations|SetCenterCandleLocation (Variables|/Script/Engine.SceneComponent|GetRelativeLocation (Variables|Default|GetCenterCandle)))
  (Variables|Locations|SetRightCandleLocation (Variables|/Script/Engine.SceneComponent|GetRelativeLocation (Variables|Default|GetRightCandle)))
  (Variables|Locations|SetLeftForkLocation (Variables|/Script/Engine.SceneComponent|GetRelativeLocation (Variables|Default|GetLeftFork)))
  (Variables|Locations|SetCenterForkLocation (Variables|/Script/Engine.SceneComponent|GetRelativeLocation (Variables|Default|GetCenterFork)))
  (Variables|Locations|SetRightForkLocation (Variables|/Script/Engine.SceneComponent|GetRelativeLocation (Variables|Default|GetRightFork)))
  (Variables|Locations|SetLeftBearLocation (Variables|/Script/Engine.SceneComponent|GetRelativeLocation (Variables|Default|GetLeftBear)))
  (Variables|Locations|SetRightBearLocation (Variables|/Script/Engine.SceneComponent|GetRelativeLocation (Variables|Default|GetRightBear))))