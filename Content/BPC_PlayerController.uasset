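; Player controller Blueprint that moves the controlled pawn sideways between lanes on touch input.
; A first-finger press in the right or left third of the viewport shifts the pawn one lane along Y, unless it is already at that side's limit.
; Delayed for-loop macros split each shift into small, timed world offsets without sweep, while an IsMoving flag blocks new presses until it completes.
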(event Input|TouchEvents|InputTouch
  (params (Location :type Vector) (FingerIndex :type ETouchIndex%20Enum))
  (bind _returnvalue (Pawn|GetControlledPawn))
  (bind _x (Math|Vector|BreakVector Location))
  (bind _returnvalue_2 (Game|GetPlayerController 0))
  (bind _returnvalue_3 (Utilities|Enum|Equal(Enum) FingerIndex "Touch1"))
  (bind _sizex (HUD|GetViewportSize _returnvalue_2))
  (:Pressed
    (if (not (Variables|Default|GetisMoving))
      (if (and _returnvalue_3 (>= _x (* _sizex 0.667)))
        (if (!= (.y (Transformation|GetActorLocation _returnvalue)) 4e+02)
          (Utilities|ForLoopDelay 0 9 :!label _label
            (:Loop%20Body
              (Variables|Default|SetisMoving true)
              (Transformation|AddActorWorldOffset (Pawn|GetControlledPawn) "0,40.000000,0.000000"))
            (:Completed
              (Variables|Default|SetisMoving false))
            (:Delay%20Out
              (Utilities|FlowControl|Delay 0.001)
              (goto _label Delay%20In))))
        (elif (and _returnvalue_3 (<= _x (* _sizex 0.334)))
          (if (!= (.y (Transformation|GetActorLocation _returnvalue)) -4e+02)
            (Utilities|ForLoopDelay 0 9 :!label _label_2
              (:Loop%20Body
                (Variables|Default|SetisMoving true)
                (Transformation|AddActorWorldOffset (Pawn|GetControlledPawn) "0,-40.000000,0.000000"))
              (:Completed
                (Variables|Default|SetisMoving false))
              (:Delay%20Out
                (Utilities|FlowControl|Delay 0.001)
                (goto _label_2 Delay%20In)))))))))

(fn ConstructionScript)